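; Behavior tree service that keeps an AI enemy's distance to its target object up to date on the blackboard.
; Each tick it reads the target actor key and measures the horizontal distance from the controlled pawn, ignoring height.
; The result goes to the distance key, or zero when no valid target exists, so a missing target reads the same as being on top of it.
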(event EventTick
  (params (OwnerActor :type Actor%20Object%20Reference) (DeltaSeconds :type Float%20%28single-precision%29))
  (bind _targetobjectkey (Variables|Default|GetTargetObjectKey))
  (bind _returnvalue (AI|BehaviorTree|GetBlackboardValueasActor _targetobjectkey))
  (bind _returnvalue_2 (Transformation|GetActorLocation _returnvalue))
  (bind (_x _y) (Math|Vector|BreakVector _returnvalue_2))
  (bind _asaienemy_controller (Utilities|Casting|CastToAIEnemyController OwnerActor))
  (Utilities|IsValid _returnvalue
    (:Is%20Valid
      (Class|BTFunctionLibrary|SetBlackboardValueasFloat (Variables|Default|GetTargetObjectDistanceKey) (Math|Vector|VectorLength (- (Math|Vector|MakeVector (.X (Math|Vector|BreakVector (Transformation|GetActorLocation (Pawn|GetControlledPawn _asaienemy_controller)))) (.Y (Math|Vector|BreakVector (Transformation|GetActorLocation (Pawn|GetControlledPawn _asaienemy_controller)))) 0.0) (Math|Vector|MakeVector _x _y 0.0)))))
    (:Is%20Not%20Valid
      (Class|BTFunctionLibrary|SetBlackboardValueasFloat (Variables|Default|GetTargetObjectDistanceKey) 0.0))))