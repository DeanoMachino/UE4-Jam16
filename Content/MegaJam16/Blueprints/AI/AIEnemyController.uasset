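; AI controller for enemies that starts the AIEnemyBT behavior tree on BeginPlay.
; A PawnSensing component feeds the blackboard: any seen pawn is stored as the enemy actor, with no filtering.
; Heard noises within a fixed distance of the controlled pawn set an investigate position and a heard-noise flag.
; Both sensing events also print debug messages to the screen.
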(event OnSeePawn(PawnSensing)
  (params (Pawn :type Pawn%20Object%20Reference))
  (Development|PrintString "AI saw a pawn" true true "(R=1.000000,G=0.000000,B=0.660178,A=1.000000)")
  (AI|Components|Blackboard|SetValueasObject (AI|GetBlackboard self) (Variables|Default|GetEnemyActorKeyName) Pawn))

(event OnHearNoise(PawnSensing)
  (params (Instigator :type Pawn%20Object%20Reference) (Location :type Vector%20%28by%20ref%29) (Volume :type Float%20%28single-precision%29))
  (bind _self self)
  (bind _returnvalue (AI|GetBlackboard _self))
  (Development|PrintString "AI heard a noise" true true "(R=1.000000,G=0.000000,B=0.660178,A=1.000000)")
  (if (< (Math|Vector|VectorLength (- Location (Pawn|GetNavAgentLocation (Pawn|GetControlledPawn)))) 1e+03)
    (AI|Components|Blackboard|SetValueasVector _returnvalue (Variables|Default|GetInvestigatePositionKeyName) Location)
    (AI|Components|Blackboard|SetValueasBool _returnvalue (Variables|Default|GetHeardNoiseBoolName) true)))

(event EventBeginPlay
  (AI|RunBehaviorTree "/Game/MegaJam16/Blueprints/AI/AIEnemyBT.AIEnemyBT"))

(event EventTick
  (params (DeltaSeconds :type Float%20%28single-precision%29)))

(fn ConstructionScript)