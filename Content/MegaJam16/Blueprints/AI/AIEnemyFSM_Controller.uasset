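; AI controller for a stealth-style enemy that patrols, investigates noises and sightings, then chases and destroys the seen pawn up close.
; Runs a behavior tree but drives its five-state enum FSM itself, writing state, waypoints and investigation positions to the blackboard.
; PawnSensing and Tick dispatch per state; sightings raise a decaying suspicion level by proximity, with thresholds triggering investigation or chase.
; Volume-scaled noises trigger investigation; patrol waypoints loop.
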(event OnSeePawn(PawnSensing)
  (params (Pawn :type Pawn%20Object%20Reference))
  ;[1 1 1] On See Pawn
  (bind _output_get (Variables|SenseDetection|SetSeenPawn Pawn))
  (bind _isinrange_ (SenseDetection|CheckIsinRange _output_get (Variables|SenseDetection|GetSightRange)))
  (if _isinrange_
    (bind _aienemystate (Behaviour|GetAIEnemyState (AI|GetBlackboard 0)))
    (switch Utilities|FlowControl|Switch|SwitchonAIEnemyFSM_AIState _aienemystate
      (:NewEnumerator0
        (CallFunction|OnSeePawnIdle))
      (:NewEnumerator1
        (CallFunction|OnSeePawnPatrolling))
      (:NewEnumerator3
        (CallFunction|OnSeePawnInvestigatingNoise))
      (:NewEnumerator2
        (CallFunction|OnSeePawnInvestigatingSight))
      (:NewEnumerator4
        (CallFunction|OnSeePawnChasingPlayer)))))

(event OnHearNoise(PawnSensing)
  (params (Instigator :type Pawn%20Object%20Reference) (Location :type Vector%20%28by%20ref%29) (Volume :type Float%20%28single-precision%29))
  ;[1 1 1] On Hear Noise
  (bind _isinrange_ (SenseDetection|CheckIsinRange Instigator (* Volume (Variables|SenseDetection|GetHearingRange))))
  (if _isinrange_
    (Variables|Default|SetNoiseLocation Location)
    (bind _aienemystate (Behaviour|GetAIEnemyState (AI|GetBlackboard 0)))
    (switch Utilities|FlowControl|Switch|SwitchonAIEnemyFSM_AIState _aienemystate
      (:NewEnumerator0
        (CallFunction|OnHearNoiseIdle))
      (:NewEnumerator1
        (CallFunction|OnHearNoisePatrolling))
      (:NewEnumerator3
        (CallFunction|OnHearNoiseInvestigatingNoise))
      (:NewEnumerator2
        (CallFunction|OnHearNoiseInvestigatingSight))
      (:NewEnumerator4
        (CallFunction|OnHearNoiseChasingPlayer)))))

(event Custom|OnSeePawn_Idle
  (bind _sightrange (Variables|SenseDetection|GetSightRange))
  (bind _distance (CallFunction|GetDistanceBetweenPawnandAI))
  (SenseDetection|IncrementSuspicionLevel (/ (/ (- _sightrange _distance) _sightrange) 15.0)))

(event Custom|EventTick_Idle
  (bind _returnvalue (AI|GetBlackboard 0))
  ;[1 1 1] Event Tick -- Idle
  (Utilities|FlowControl|Sequence
    (:then_0
      (SenseDetection|IncrementSuspicionLevel -0.01)
      (SenseDetection|CheckifShouldInvestigateSight _returnvalue))
    (:then_1
      (PatrolRoute|CheckifShouldbePatrolling _returnvalue))))

(event Custom|OnSeePawn_InvestigatingSight
  (bind _sightrange (Variables|SenseDetection|GetSightRange))
  (bind _distance (CallFunction|GetDistanceBetweenPawnandAI))
  (SenseDetection|IncrementSuspicionLevel (/ (/ (- _sightrange _distance) _sightrange) 15.0)))

(event Custom|EventTick_Patrolling
  ;[1 1 1] Event Tick -- Patrolling
  (Utilities|FlowControl|Sequence
    (:then_0
      (PatrolRoute|ChangePatrolWaypoint (AI|GetBlackboard 0)))
    (:then_1
      (CallFunction|EventTickIdle))))

(event Custom|EventTick_InvestigatingNoise
  (bind _returnvalue (AI|GetBlackboard 0))
  (Utilities|FlowControl|Sequence
    (:then_0
      (bind _outputvalue (BlackboardUtilities|GetBlackboardBool _returnvalue (Variables|BlackboardKeys|GetHasHeardNoiseKeyName)))
      (if (not _outputvalue)
        (Behaviour|SetAIEnemyState _returnvalue "NewEnumerator0")))
    (:then_1
      (CallFunction|EventTickIdle))))

(event Custom|OnSeePawn_ChasingPlayer
  (bind _sightrange (Variables|SenseDetection|GetSightRange))
  (Utilities|FlowControl|Sequence
    (:then_0
      (bind _distance (CallFunction|GetDistanceBetweenPawnandAI))
      (SenseDetection|IncrementSuspicionLevel (/ (/ (- _sightrange _distance) _sightrange) 15.0)))
    (:then_1
      (BlackboardUtilities|SetBlackboardVector (AI|GetBlackboard 0) (Variables|BlackboardKeys|GetInvestigationPositionKeyName) (Transformation|GetActorLocation (Variables|SenseDetection|GetSeenPawn))))))

(event Custom|EventTick_InvestigatingSight
  (bind _returnvalue (AI|GetBlackboard 0))
  ;[1 1 1] Event Tick -- Investigating Sight
  (SenseDetection|IncrementSuspicionLevel -0.01)
  (Utilities|CheckifSuspicionLevelIsAboveValue 1.0
    (:True
      (Behaviour|SetAIEnemyState _returnvalue "NewEnumerator4")
      (BlackboardUtilities|SetBlackboardVector _returnvalue (Variables|BlackboardKeys|GetInvestigationPositionKeyName) (Transformation|GetActorLocation (Variables|SenseDetection|GetSeenPawn))))))

(event Custom|EventTick_ChasingPawn
  (bind _seenpawn (Variables|SenseDetection|GetSeenPawn))
  (Utilities|FlowControl|Sequence
    (:then_0
      (SenseDetection|IncrementSuspicionLevel -0.01)
      (Utilities|CheckifSuspicionLevelIsBelowValue 0.1
        (:True
          (Behaviour|SetAIEnemyState (AI|GetBlackboard 0) "NewEnumerator0"))))
    (:then_1
      (bind _isinrange_ (SenseDetection|CheckIsinRange _seenpawn 1.5e+02))
      (if _isinrange_
        (Actor|DestroyActor _seenpawn)))))

(event Custom|OnHearNoise_Idle
  (bind _returnvalue (AI|GetBlackboard 0))
  (Behaviour|SetAIEnemyState _returnvalue "NewEnumerator3")
  (BlackboardUtilities|SetBlackboardVector _returnvalue (Variables|BlackboardKeys|GetInvestigationPositionKeyName) (Variables|Default|GetNoiseLocation))
  (BlackboardUtilities|SetBlackboardBool _returnvalue (Variables|BlackboardKeys|GetHasHeardNoiseKeyName) true)
  (Development|PrintString "AI Heard Noise" true true "(R=0.000000,G=0.660000,B=1.000000,A=1.000000)" 0.01))

(event Custom|OnSeePawn_Patrolling
  (bind _sightrange (Variables|SenseDetection|GetSightRange))
  (bind _distance (CallFunction|GetDistanceBetweenPawnandAI))
  (SenseDetection|IncrementSuspicionLevel (/ (/ (- _sightrange _distance) _sightrange) 15.0)))

(event Custom|OnHearNoise_Patrolling
  (bind _returnvalue (AI|GetBlackboard 0))
  (Behaviour|SetAIEnemyState _returnvalue "NewEnumerator3")
  (BlackboardUtilities|SetBlackboardVector _returnvalue (Variables|BlackboardKeys|GetInvestigationPositionKeyName) (Variables|Default|GetNoiseLocation))
  (BlackboardUtilities|SetBlackboardBool _returnvalue (Variables|BlackboardKeys|GetHasHeardNoiseKeyName) true)
  (Development|PrintString "AI Heard Noise" true true "(R=0.000000,G=0.660000,B=1.000000,A=1.000000)" 0.01))

(event Custom|OnHearNoise_InvestigatingNoise
  (bind _returnvalue (AI|GetBlackboard 0))
  (Behaviour|SetAIEnemyState _returnvalue "NewEnumerator3")
  (BlackboardUtilities|SetBlackboardVector _returnvalue (Variables|BlackboardKeys|GetInvestigationPositionKeyName) (Variables|Default|GetNoiseLocation))
  (BlackboardUtilities|SetBlackboardBool _returnvalue (Variables|BlackboardKeys|GetHasHeardNoiseKeyName) true)
  (Development|PrintString "AI Heard Noise" true true "(R=0.000000,G=0.660000,B=1.000000,A=1.000000)" 0.01))

(event Custom|OnHearNoise_InvestigatingSight)

(event Custom|OnHearNoise_ChasingPlayer)

(event Custom|OnSeePawn_InvestigatingNoise
  (bind _sightrange (Variables|SenseDetection|GetSightRange))
  (bind _distance (CallFunction|GetDistanceBetweenPawnandAI))
  (SenseDetection|IncrementSuspicionLevel (/ (/ (- _sightrange _distance) _sightrange) 15.0)))

(event EventBeginPlay
  (bind _returnvalue (AI|GetBlackboard 0))
  (bind _waypointpositions (Variables|PatrolRoute|GetWaypointPositions))
  (bind _waypointrotations (Variables|PatrolRoute|GetWaypointRotations))
  ;[1 1 1] Event BeginPlay
  (|CallParentFunction)
  (AI|RunBehaviorTree "/Game/MegaJam16/Blueprints/AI/AIEnemyFSM_BT.AIEnemyFSM_BT")
  (Behaviour|SetAIEnemyState _returnvalue "NewEnumerator0") ; Initialise the AIEnemy state
  (bind _outputvalue (BlackboardUtilities|SetBlackboardBool _returnvalue (Variables|BlackboardKeys|GetHasPatrolRouteKeyName) true)) ; Initialise whether the AI has a patrol route or not
  (if _outputvalue ; If the AI has a patrol route
    (bind _asaienemy_fsm_character (Utilities|Casting|CastToAIEnemyFSM_Character (Pawn|GetControlledPawn)))
    (for _array_element (Variables|/Game/MegaJam16/Blueprints/AI/AIEnemyFSM_Character.AIEnemyFSM_Character_C|GetPatrolWaypointArray _asaienemy_fsm_character)
      (Utilities|Array|Add _waypointpositions (Transformation|GetActorLocation _array_element))
      (Utilities|Array|Add _waypointrotations (Transformation|GetActorRotation _array_element)))
    (bind _output_get (Variables|PatrolRoute|SetWaypointIndex 0))
    (BlackboardUtilities|SetBlackboardVector _returnvalue (Variables|BlackboardKeys|GetCurrentWaypointPositionKeyName) (Utilities|Array|Get(acopy) _waypointpositions _output_get)) ; Set current waypoint
    (BlackboardUtilities|SetBlackboardRotator _returnvalue (Variables|BlackboardKeys|GetCurrentWaypointRotationKeyName) (Utilities|Array|Get(acopy) _waypointrotations _output_get)) ; Set current waypoint rotation
  ))

(event EventTick
  (params (DeltaSeconds :type Float%20%28single-precision%29))
  ;[1 1 1] Event Tick
  (bind _aienemystate (Behaviour|GetAIEnemyState (AI|GetBlackboard 0)))
  (switch Utilities|FlowControl|Switch|SwitchonAIEnemyFSM_AIState _aienemystate
    (:NewEnumerator0
      (CallFunction|EventTickIdle))
    (:NewEnumerator1
      (CallFunction|EventTickPatrolling))
    (:NewEnumerator3
      (CallFunction|EventTickInvestigatingNoise))
    (:NewEnumerator2
      (CallFunction|EventTickInvestigatingSight))
    (:NewEnumerator4
      (CallFunction|EventTickChasingPawn))))

(fn ConstructionScript
  (|CallParentFunction))

(fn SetAIEnemyState
  (params (Blackboard :type Blackboard%20Component%20Object%20Reference) (AIEnemyState :type AIEnemyFSM_AIState%20Enum))
  (AI|Navigation|StopMovement)
  (AI|Components|Blackboard|SetValueasEnum Blackboard (Variables|BlackboardKeys|GetAIEnemyStateKeyName) AIEnemyState)
  (Development|PrintString (Utilities|String|Append "New EnemyState: " (Utilities|String|EnumtoString AIEnemyState)) true false "(R=1.000000,G=0.300000,B=0.000000,A=1.000000)")
  (return))

(fn IncrementSuspicionLevel
  (params (IncrementAmount :type Float%20%28single-precision%29))
  (bind _output_get (Variables|SenseDetection|SetSuspicionLevel (Math|Float|Clamp(Float) (+ IncrementAmount (Variables|SenseDetection|GetSuspicionLevel)) 0.0 1.1)))
  (Development|PrintString (Utilities|String|Append "SuspicionLevel: " (Utilities|String|ToString(Float) (Math|Float|Clamp(Float) (+ IncrementAmount (Variables|SenseDetection|GetSuspicionLevel)) 0.0 1.1))) true false "(R=1.000000,G=0.000000,B=0.403795,A=1.000000)" 0.01)
  (return _output_get))

(fn SetBlackboardFloat
  (params (Blackboard :type Blackboard%20Component%20Object%20Reference) (BlackboardKey :type Name) (Value :type Float%20%28single-precision%29))
  (AI|Components|Blackboard|SetValueasFloat Blackboard BlackboardKey Value)
  (return Value))

(fn SetBlackboardBool
  (params (Blackboard :type Blackboard%20Component%20Object%20Reference) (BlackboardKey :type Name) (Value :type Boolean))
  (AI|Components|Blackboard|SetValueasBool Blackboard BlackboardKey Value)
  (return Value))

(fn SetBlackboardInt
  (params (Blackboard :type Blackboard%20Component%20Object%20Reference) (BlackboardKey :type Name) (Value :type Integer))
  (Class|BlackboardComponent|SetValueasInt Blackboard BlackboardKey Value)
  (return Value))

(fn CheckIsinRange
  (params (Pawn :type Pawn%20Object%20Reference) (Range :type Float%20%28single-precision%29))
  (return (< (Math|Vector|VectorLength (- (Transformation|GetActorLocation Pawn) (Pawn|GetNavAgentLocation (Pawn|GetControlledPawn)))) Range)))

(fn SetBlackboardVector
  (params (Blackboard :type Blackboard%20Component%20Object%20Reference) (BlackboardKey :type Name) (Value :type Vector))
  (AI|Components|Blackboard|SetValueasVector Blackboard BlackboardKey Value)
  (return Value))

(fn GetBlackboardFloat
  (params (Blackboard :type Blackboard%20Component%20Object%20Reference) (BlackboardKey :type Name))
  (return (Class|BlackboardComponent|GetValueasFloat Blackboard BlackboardKey)))

(fn GetBlackboardBool
  (params (Blackboard :type Blackboard%20Component%20Object%20Reference) (BlackboardKey :type Name))
  (return (ScalableFloat|GetValueasBool Blackboard BlackboardKey)))

(fn GetBlackboardInt
  (params (Blackboard :type Blackboard%20Component%20Object%20Reference) (BlackboardKey :type Name))
  (return (Class|BlackboardComponent|GetValueasInt Blackboard BlackboardKey)))

(fn GetBlackboardVector
  (params (Blackboard :type Blackboard%20Component%20Object%20Reference) (BlackboardKey :type Name))
  (return (AI|Components|Blackboard|GetValueasVector Blackboard BlackboardKey)))

(fn GetAIEnemyState
  (params (Blackboard :type Blackboard%20Component%20Object%20Reference))
  (return (Utilities|Enum|ByteToEnumAIEnemyFSM_AIState (Class|BlackboardComponent|GetValueasEnum Blackboard (Variables|BlackboardKeys|GetAIEnemyStateKeyName)))))

(fn ChangePatrolWaypoint
  (params (Blackboard :type Blackboard%20Component%20Object%20Reference))
  (bind _waypointpositions (Variables|PatrolRoute|GetWaypointPositions))
  (bind _outputvalue (BlackboardUtilities|GetBlackboardBool Blackboard (Variables|BlackboardKeys|GetArrivedAtWaypoint)))
  (if _outputvalue
    (bind _result (Math|Integer|IncrementInt (Variables|PatrolRoute|GetWaypointIndex))
      (:%20%20
        (bind _output_get (Variables|PatrolRoute|SetWaypointIndex (Math|Integer|SelectInt 0 _result (>= _result (Utilities|Array|Length _waypointpositions)))))
        (BlackboardUtilities|SetBlackboardVector Blackboard (Variables|BlackboardKeys|GetCurrentWaypointPositionKeyName) (Utilities|Array|Get(acopy) _waypointpositions _output_get))
        (BlackboardUtilities|SetBlackboardRotator Blackboard (Variables|BlackboardKeys|GetCurrentWaypointRotationKeyName) (Utilities|Array|Get(acopy) (Variables|PatrolRoute|GetWaypointRotations) _output_get))
        (BlackboardUtilities|SetBlackboardBool Blackboard (Variables|BlackboardKeys|GetArrivedAtWaypoint) false))))
  (return _outputvalue))

(fn CheckifShouldbePatrolling
  (params (Blackboard :type Blackboard%20Component%20Object%20Reference))
  (bind _outputvalue (BlackboardUtilities|GetBlackboardBool Blackboard (Variables|BlackboardKeys|GetHasPatrolRouteKeyName)))
  (bind _aienemystate (Behaviour|GetAIEnemyState Blackboard))
  (if (and (Utilities|Enum|Equal(Enum) _aienemystate "NewEnumerator0") _outputvalue)
    (Behaviour|SetAIEnemyState Blackboard "NewEnumerator1"))
  (return (and (Utilities|Enum|Equal(Enum) _aienemystate "NewEnumerator0") _outputvalue)))

(fn CheckifShouldInvestigateSight
  (params (Blackboard :type Blackboard%20Component%20Object%20Reference))
  (bind _result (Utilities|CheckifSuspicionLevelIsAboveValue 0.5)
    (:True
      (Behaviour|SetAIEnemyState Blackboard "NewEnumerator2")
      (BlackboardUtilities|SetBlackboardVector Blackboard (Variables|BlackboardKeys|GetInvestigationPositionKeyName) (Transformation|GetActorLocation (Variables|SenseDetection|GetSeenPawn))))
    (:False
      _))
  (return _result))

(fn GetDistanceBetweenPawnandAI
  (return (Math|Vector|VectorLength (- (Transformation|GetActorLocation (Variables|SenseDetection|GetSeenPawn)) (Pawn|GetNavAgentLocation (Pawn|GetControlledPawn))))))

(fn SetBlackboardRotator
  (params (Blackboard :type Blackboard%20Component%20Object%20Reference) (BlackboardKey :type Name) (Value :type Rotator))
  (Class|BlackboardComponent|SetValueasRotator Blackboard BlackboardKey Value)
  (return Value))

(fn GetBlackboardRotator
  (params (Blackboard :type Blackboard%20Component%20Object%20Reference) (BlackboardKey :type Name))
  (return (Class|BlackboardComponent|GetValueasRotator Blackboard BlackboardKey)))