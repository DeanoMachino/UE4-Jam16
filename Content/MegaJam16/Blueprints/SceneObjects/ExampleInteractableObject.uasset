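; Example interactable physics object that reacts to interaction and throwing, and makes noise on hard impacts.
; Interacting pops the sphere upward, while throwing launches it along the given forward vector; both spawn an explosion particle.
; A throw sets a Thrown flag, so the first hit above a speed threshold emits a noise event at the hit location, then clears the flag.
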(event EventBeginPlay)

(event Collision|EventActorBeginOverlap
  (params (OtherActor :type Actor%20Object%20Reference)))

(event Collision|EventHit
  (params (MyComp :type Primitive%20Component%20Object%20Reference) (Other :type Actor%20Object%20Reference) (OtherComp :type Primitive%20Component%20Object%20Reference) (bSelfMoved :type Boolean) (HitLocation :type Vector) (HitNormal :type Vector :default "0, 0, 0") (NormalImpulse :type Vector :default "0, 0, 0") (Hit :type Hit%20Result%20Structure%20%28by%20ref%29))
  (if (Variables|Default|GetThrown)
    (if (> (Math|Vector|VectorLength (Transformation|GetComponentVelocity (Variables|Default|GetSphere))) 1.5e+03)
      (Class|Actor|MakeNoise 1.0 self HitLocation 0.0 "None")
      (Variables|Default|SetThrown false))))

(event EventOnThrow
  (params (ForwardVector :type Vector))
  (Variables|Default|SetThrown true)
  (Physics|AddImpulse (Variables|Default|GetSphere) (* ForwardVector 5e+04) "None" false)
  (Effects|SpawnEmitteratLocation "/Game/StarterContent/Particles/P_Explosion.P_Explosion" (Transformation|GetWorldLocation (Variables|Default|GetSphere))))

(event EventTick
  (params (DeltaSeconds :type Float%20%28single-precision%29)))

(event EventOnInteract
  (Effects|SpawnEmitteratLocation "/Game/StarterContent/Particles/P_Explosion.P_Explosion" (Transformation|GetWorldLocation (Variables|Default|GetSphere)))
  (Physics|AddImpulse (Variables|Default|GetSphere) "0,0.000000,50000.000000" "None" false))

(fn ConstructionScript)