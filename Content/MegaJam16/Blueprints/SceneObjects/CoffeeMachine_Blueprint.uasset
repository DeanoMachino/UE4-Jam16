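; Interactable coffee machine that gradually refills the first-person character's coffee level while the player holds E inside its trigger.
; Trigger overlap enables or disables input, and E toggles an interacting flag, with release or leaving the trigger hiding the character's coffee meter widget.
; While interacting, Tick shows the meter and raises CoffeeLevel in small delayed steps up to a cap, and separately disables interactability when full.
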(event OnComponentBeginOverlap(Trigger)
  (params (OverlappedComponent :type Primitive%20Component%20Object%20Reference) (OtherActor :type Actor%20Object%20Reference) (OtherComp :type Primitive%20Component%20Object%20Reference) (OtherBodyIndex :type Integer) (bFromSweep :type Boolean) (SweepResult :type Hit%20Result%20Structure%20%28by%20ref%29))
  ;[1 1 1] Test If Can Interact
  (Input|EnableInput (Game|GetPlayerController 0)))

(event OnComponentEndOverlap(Trigger)
  (params (OverlappedComponent :type Primitive%20Component%20Object%20Reference) (OtherActor :type Actor%20Object%20Reference) (OtherComp :type Primitive%20Component%20Object%20Reference) (OtherBodyIndex :type Integer))
  ;[1 1 1] Test If Can Interact
  (Input|DisableInput (Game|GetPlayerController 0))
  ;[1 1 1] Progress Bar
  (Variables|Default|SetInteracting false)
  (bind _output_get (Variables|Default|SetCoffee_Meter (Variables|/Game/MegaJam16/Blueprints/Character/FirstPersonCharacter.FirstPersonCharacter_C|GetCoffee_Wid (Variables|Default|GetmyCharacter))))
  (Widget|SetVisibility _output_get "Hidden"))

(event EventBeginPlay
  (Variables|Default|SetCoffeeVal 0.0)
  (bind _asfirst_person_character (Utilities|Casting|CastToFirstPersonCharacter (Game|GetPlayerCharacter 0)))
  (Variables|Default|SetmyCharacter _asfirst_person_character)
  (Variables|Default|SetisInteractable true))

(event EventTick
  (params (DeltaSeconds :type Float%20%28single-precision%29))
  ;[1 1 1] Progress Bar
  (Utilities|FlowControl|Sequence
    (:then_0
      (if (Variables|Default|GetInteracting)
        (bind _asfirst_person_character (Utilities|Casting|CastToFirstPersonCharacter (Game|GetPlayerCharacter 0)))
        (Variables|Default|SetmyCharacter _asfirst_person_character)
        (bind _output_get (Variables|Default|SetCoffee_Meter (Variables|/Game/MegaJam16/Blueprints/Character/FirstPersonCharacter.FirstPersonCharacter_C|GetCoffee_Wid (Variables|Default|GetmyCharacter))))
        (Widget|SetVisibility _output_get "Visible")
        (Utilities|FlowControl|Delay 0.01)
        (if (<= (+ (Variables|/Game/MegaJam16/Blueprints/Character/FirstPersonCharacter.FirstPersonCharacter_C|GetCoffee_Level (Variables|Default|GetmyCharacter)) 0.0015) 1.0)
          (Variables|/Game/MegaJam16/Blueprints/Character/FirstPersonCharacter.FirstPersonCharacter_C|SetCoffee_Level (Variables|Default|GetmyCharacter) (+ (Variables|/Game/MegaJam16/Blueprints/Character/FirstPersonCharacter.FirstPersonCharacter_C|GetCoffee_Level (Variables|Default|GetmyCharacter)) 0.0015))
          (else
            (Variables|/Game/MegaJam16/Blueprints/Character/FirstPersonCharacter.FirstPersonCharacter_C|SetCoffee_Level (Variables|Default|GetmyCharacter) 1.0)))))
    (:then_1
      (if (< (Variables|/Game/MegaJam16/Blueprints/Character/FirstPersonCharacter.FirstPersonCharacter_C|GetCoffee_Level (Variables|Default|GetmyCharacter)) 1.0)
        (Variables|Default|SetisInteractable true)
        (else
          (Variables|Default|SetisInteractable false))))))

(event Input|KeyboardEvents|E
  (params (Key :type Key%20Structure :default "AnyKey"))
  ;[1 1 1] Progress Bar
  (:Pressed
    (if (Variables|Default|GetisInteractable)
      (Variables|Default|SetInteracting true)
      (else
        (Variables|Default|SetInteracting false)
        (Widget|SetVisibility (stale _output_get) "Hidden" :!label _label))))
  (:Released
    (Variables|Default|SetInteracting false)
    (bind _output_get (Variables|Default|SetCoffee_Meter (Variables|/Game/MegaJam16/Blueprints/Character/FirstPersonCharacter.FirstPersonCharacter_C|GetCoffee_Wid (Variables|Default|GetmyCharacter))))
    (goto _label)))

(fn ConstructionScript)