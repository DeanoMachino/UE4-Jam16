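; Interactable scene object that the player works on by holding E inside its trigger, spending coffee to build progress.
; Trigger overlap toggles input on the actor, while release or exit stops interacting and hides the character's progress and coffee widgets.
; Tick shows both widgets and, through a short Delay, raises progress and drains CoffeeLevel in fixed steps.
; Interaction locks when coffee is empty or progress is full, with no completion action wired.
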(event OnComponentBeginOverlap(Trigger)
  (params (OverlappedComponent :type Primitive%20Component%20Object%20Reference) (OtherActor :type Actor%20Object%20Reference) (OtherComp :type Primitive%20Component%20Object%20Reference) (OtherBodyIndex :type Integer) (bFromSweep :type Boolean) (SweepResult :type Hit%20Result%20Structure%20%28by%20ref%29))
  ;[1 1 1] Test If Can Interact
  (Input|EnableInput (Game|GetPlayerController 0)))

(event OnComponentEndOverlap(Trigger)
  (params (OverlappedComponent :type Primitive%20Component%20Object%20Reference) (OtherActor :type Actor%20Object%20Reference) (OtherComp :type Primitive%20Component%20Object%20Reference) (OtherBodyIndex :type Integer))
  (bind _mycharacter (Variables|Default|GetmyCharacter))
  ;[1 1 1] Test If Can Interact
  (Input|DisableInput (Game|GetPlayerController 0))
  ;[1 1 1] Progress Bar
  (Variables|Default|SetInteracting false)
  (bind _output_get (Variables|Default|SetProgress_Bar (Variables|/Game/MegaJam16/Blueprints/Character/FirstPersonCharacter.FirstPersonCharacter_C|GetProg_Wid _mycharacter)))
  (Widget|SetVisibility _output_get "Hidden")
  (bind _output_get_2 (Variables|Default|SetCoffee_Meter (Variables|/Game/MegaJam16/Blueprints/Character/FirstPersonCharacter.FirstPersonCharacter_C|GetCoffee_Wid _mycharacter)))
  (Widget|SetVisibility _output_get_2 "Hidden"))

(event EventBeginPlay
  (Variables|Default|SetProgressComp 0.0)
  (Variables|Default|SetCoffeeVal 0.0)
  (bind _asfirst_person_character (Utilities|Casting|CastToFirstPersonCharacter (Game|GetPlayerCharacter 0)))
  (Variables|Default|SetmyCharacter _asfirst_person_character)
  (Variables|Default|SetisInteractable true))

(event EventTick
  (params (DeltaSeconds :type Float%20%28single-precision%29))
  ;[1 1 1] Progress Bar
  (Utilities|FlowControl|Sequence
    (:then_0
      (if (Variables|Default|GetInteracting)
        (bind _asfirst_person_character (Utilities|Casting|CastToFirstPersonCharacter (Game|GetPlayerCharacter 0)))
        (Variables|Default|SetmyCharacter _asfirst_person_character)
        (bind _output_get (Variables|Default|SetProgress_Bar (Variables|/Game/MegaJam16/Blueprints/Character/FirstPersonCharacter.FirstPersonCharacter_C|GetProg_Wid (Variables|Default|GetmyCharacter))))
        (Variables|/Game/MegaJam16/Blueprints/UMG/ProgressBar_BP.ProgressBar_BP_C|SetCompletion (Variables|/Game/MegaJam16/Blueprints/Character/FirstPersonCharacter.FirstPersonCharacter_C|GetProg_Wid (Variables|Default|GetmyCharacter)) (Variables|Default|GetProgressComp))
        (Widget|SetVisibility _output_get "Visible")
        (bind _output_get_2 (Variables|Default|SetCoffee_Meter (Variables|/Game/MegaJam16/Blueprints/Character/FirstPersonCharacter.FirstPersonCharacter_C|GetCoffee_Wid (Variables|Default|GetmyCharacter))))
        (Widget|SetVisibility _output_get_2 "Visible")
        (Utilities|FlowControl|Delay 0.01)
        (Utilities|FlowControl|Sequence
          (:then_0
            (bind _output_get_3 (Variables|Default|SetProgressComp (+ (Variables|Default|GetProgressComp) 0.003)))
            (Variables|/Game/MegaJam16/Blueprints/UMG/ProgressBar_BP.ProgressBar_BP_C|SetCompletion (Variables|/Game/MegaJam16/Blueprints/Character/FirstPersonCharacter.FirstPersonCharacter_C|GetProg_Wid (Variables|Default|GetmyCharacter)) _output_get_3))
          (:then_1
            (if (>= (- (Variables|/Game/MegaJam16/Blueprints/Character/FirstPersonCharacter.FirstPersonCharacter_C|GetCoffee_Level (Variables|Default|GetmyCharacter)) 0.0005) 0.0)
              (Variables|/Game/MegaJam16/Blueprints/Character/FirstPersonCharacter.FirstPersonCharacter_C|SetCoffee_Level (Variables|Default|GetmyCharacter) (- (Variables|/Game/MegaJam16/Blueprints/Character/FirstPersonCharacter.FirstPersonCharacter_C|GetCoffee_Level (Variables|Default|GetmyCharacter)) 0.0005))
              (else
                (Variables|/Game/MegaJam16/Blueprints/Character/FirstPersonCharacter.FirstPersonCharacter_C|SetCoffee_Level (Variables|Default|GetmyCharacter) 0.0)))))))
    (:then_1
      (if (and (> (Variables|/Game/MegaJam16/Blueprints/Character/FirstPersonCharacter.FirstPersonCharacter_C|GetCoffee_Level (Variables|Default|GetmyCharacter)) 0.0) (< (Variables|Default|GetProgressComp) 1.0))
        (Variables|Default|SetisInteractable true)
        (else
          (Variables|Default|SetisInteractable false)
          (Variables|Default|SetInteracting false)
          (if (< (Variables|Default|GetProgressComp) 1.0)
            _))))))

(event Input|KeyboardEvents|E
  (params (Key :type Key%20Structure :default "AnyKey"))
  (bind _mycharacter (Variables|Default|GetmyCharacter))
  ;[1 1 1] Progress Bar
  (:Pressed
    (if (Variables|Default|GetisInteractable)
      (Variables|Default|SetInteracting true)
      (else
        (Variables|Default|SetInteracting false))))
  (:Released
    (Variables|Default|SetInteracting false)
    (bind _output_get (Variables|Default|SetProgress_Bar (Variables|/Game/MegaJam16/Blueprints/Character/FirstPersonCharacter.FirstPersonCharacter_C|GetProg_Wid _mycharacter)))
    (Widget|SetVisibility _output_get "Hidden")
    (bind _output_get_2 (Variables|Default|SetCoffee_Meter (Variables|/Game/MegaJam16/Blueprints/Character/FirstPersonCharacter.FirstPersonCharacter_C|GetCoffee_Wid _mycharacter)))
    (Widget|SetVisibility _output_get_2 "Hidden")))

(fn ConstructionScript)